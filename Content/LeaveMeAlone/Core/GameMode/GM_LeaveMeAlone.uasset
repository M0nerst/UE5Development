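; GM_LeaveMeAlone is the game mode that runs the match countdown and handles the two ways the game ends.
; On BeginPlay it starts a looping one-second timer that decrements GameTime and binds to the player's LMAHealthComponent death event.
; Reaching zero pauses the game and shows WBP_TimerOut, while death stops the timer, waits briefly, then pauses and shows WBP_Death.
; Both end screens switch PC_LeaveMeAlone to UI-only input with the mouse cursor visible.
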(event Custom|CustomEvent
  (bind _output_get (Variables|Default|SetGame%20Time (- (Variables|Default|GetGame%20Time) 1)))
  (if (== _output_get 0)
    (Utilities|Time|ClearandInvalidateTimerbyHandle (Variables|Default|GetGame%20Timer%20Handle))
    (Game|SetGamePaused true)
    (bind _returnvalue (UserInterface|CreateWidget "/Game/LeaveMeAlone/Widgets/UI/WBP_TimerOut.WBP_TimerOut_C"))
    (UserInterface|Viewport|AddtoViewport _returnvalue 0)
    (bind _aspc_leave_me_alone (Utilities|Casting|CastToPC_LeaveMeAlone (Game|GetPlayerController 0)))
    (Input|SetInputModeUIOnly _aspc_leave_me_alone _returnvalue "DoNotLock" false)
    (Variables|/Script/Engine.PlayerController|SetbShowMouseCursor _aspc_leave_me_alone true)))

(event Custom|StopTimer
  (if true
    (Utilities|Time|ClearandInvalidateTimerbyHandle (Variables|Default|GetGame%20Timer%20Handle))
    (Utilities|FlowControl|Delay 2.0)
    (Game|SetGamePaused true)
    (bind _returnvalue (UserInterface|CreateWidget "/Game/LeaveMeAlone/Widgets/UI/WBP_Death.WBP_Death_C"))
    (UserInterface|Viewport|AddtoViewport _returnvalue 0)
    (bind _aspc_leave_me_alone (Utilities|Casting|CastToPC_LeaveMeAlone (Game|GetPlayerController 0)))
    (Input|SetInputModeUIOnly _aspc_leave_me_alone _returnvalue "DoNotLock" false)
    (Variables|/Script/Engine.PlayerController|SetbShowMouseCursor _aspc_leave_me_alone true)))

(event EventBeginPlay
  (bind _returnvalue (Utilities|Time|SetTimerbyEvent (delegate Custom|CustomEvent) 1.0 true))
  (Variables|Default|SetGame%20Timer%20Handle _returnvalue)
  (EventDispatchers|BindEventtoOnDeath (Actor|GetComponentbyClass (Game|GetPlayerCharacter 0) "/Script/LeaveMeAlone.LMAHealthComponent") (delegate Custom|StopTimer)))

(event EventTick
  (params (DeltaSeconds :type Float%20%28single-precision%29)))

(fn ConstructionScript)